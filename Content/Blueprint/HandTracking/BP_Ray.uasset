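; BP_Ray is an actor that displays a hand-tracking pointer ray for the hand set by HandType.
; Each Tick it shows itself only while hand tracking is the active input, the ray is valid and Enable is set.
; Pinch strength drives a morph target on the Ray mesh.
; A full pinch switches between two state materials, with a new dynamic material instance created every visible frame.
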(event EventBeginPlay)

(event EventTick
  (params (DeltaSeconds :type Float%20%28single-precision%29))
  (bind _returnvalue (Class|PICOXRInputFunctionLibrary|IsHandTrackingEnabled))
  (bind _returnvalue_2 (Class|PICOXRInputFunctionLibrary|GetActiveInputDevice))
  (bind _ray (Variables|Default|GetRay))
  (bind _handtype (Variables|Default|GetHandType))
  (bind _handtype_2 (Variables|Default|GetHandType))
  (bind _enable (Variables|Default|GetEnable))
  (bind _returnvalue_3 (Class|PICOXRInputFunctionLibrary|IsRayValid _handtype_2))
  (bind _returnvalue_4 (Class|PICOXRInputFunctionLibrary|GetPinchStrength _handtype))
  (bind _returnvalue_5 (Utilities|Enum|Equal(Enum) _returnvalue_2 "HandTrackingActive"))
  (bind _returnvalue_6 (and _returnvalue_3 _enable))
  (bind _returnvalue_7 (and _returnvalue _returnvalue_5))
  (bind _returnvalue_8 (and _returnvalue_7 _returnvalue_6))
  ;[1 1 1] UpdateRayDisplay
  (Rendering|SetActorHiddenInGame (Math|Boolean|NotEqual(Boolean) _returnvalue_8 true))
  (if _returnvalue_8
    (Components|SkeletalMesh|SetMorphTarget _ray "姿态_0" _returnvalue_4 true)
    (if (!= _returnvalue_4 1.0)
      (Rendering|Material|CreateDynamicMaterialInstance _ray 0 "/Game/Materials/Hand/MI_RaymatState1.MI_RaymatState1" "None" :!class /Script/Engine.PrimitiveComponent)
      (else
        (Rendering|Material|CreateDynamicMaterialInstance _ray 0 "/Game/Materials/Hand/MI_RaymatState2.MI_RaymatState2" "None" :!class /Script/Engine.PrimitiveComponent)))))

(fn ConstructionScript)