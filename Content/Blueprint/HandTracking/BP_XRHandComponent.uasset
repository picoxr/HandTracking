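; BP_XRHandComponent is an XR hand-tracking component that gives its owner a pointing ray for the hand set by its skeleton type.
; After a short delay on BeginPlay, if hand tracking and the ray option are on, it spawns a hidden BP_Ray, attaches it to the owner and enables it.
; While tracking is enabled, Tick moves the ray to that hand's ray pose as a relative transform.
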(event EventBeginPlay
  ;[1 1 1] init Ray
  (Utilities|FlowControl|Delay 1.0)
  (if (and (Class|PICOXRInputFunctionLibrary|IsHandTrackingEnabled) (Variables|Default|GetEnableRay))
    (bind _returnvalue (Game|SpawnActorfromClass "/Game/Blueprint/HandTracking/BP_Ray.BP_Ray_C" (Math|Transform|MakeTransform "0, 0, 0") "DontSpawnIfColliding" "OverrideRootScale" 0 0))
    (Transformation|AttachActorToActor _returnvalue (Components|GetOwner) "None" "KeepRelative" "KeepRelative" "KeepRelative" true)
    (Rendering|SetActorHiddenInGame _returnvalue true)
    (Variables|Default|SetRay _returnvalue)
    (Variables|/Game/Blueprint/HandTracking/BP_Ray.BP_Ray_C|SetHandType _returnvalue (Variables|Default|GetSkeletonType))
    (Variables|/Game/Blueprint/HandTracking/BP_Ray.BP_Ray_C|SetEnable _returnvalue true)))

(event EventTick
  (params (DeltaSeconds :type Float%20%28single-precision%29))
  (bind _ray (Variables|Default|GetRay))
  ;[1 1 1] init Ray
  (if (Class|PICOXRInputFunctionLibrary|IsHandTrackingEnabled)
    (Utilities|IsValid _ray
      (:Is%20Valid
        (Transformation|SetActorRelativeTransform _ray (Class|PICOXRInputFunctionLibrary|GetRayPose (Variables|Default|GetSkeletonType)) false false)))))